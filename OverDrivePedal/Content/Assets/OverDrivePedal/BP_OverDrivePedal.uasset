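; Interactive overdrive pedal actor that plays captured audio through a power switch and level control.
; Pressing plays a montage, then toggles power and the LED's emissive material parameter.
; Level, Drive and Tone knobs are selectable, but turning only changes level, which scales capture volume on each envelope update while powered.
; FFT output analysis runs, but its sampled magnitudes are unused and the smoothing function is a stub.
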(event `SelectLevelKnob`
  ;[0 0 0] Select Knob
  (bind _output_get (set `self.Knobs` "NewEnumerator0")))

(event `self.ReceiveBeginPlay`
  ;[0 0 0] Init FFT analyzation
  (`AudioMixerBlueprintLibrary.StartAnalyzingOutput` null "VeryLarge" "NearestNeighbor"))

(event `SelectDriveKnob`
  ;[0 0 0] Select Knob
  (bind _output_get (set `self.Knobs` "NewEnumerator1")))

(event `SelectToneKnob`
  ;[0 0 0] Select Knob
  (bind _output_get (set `self.Knobs` "NewEnumerator2")))

(event `KnobTurnLeft`
  (set `self.levelValue` (`KismetMathLibrary.FClamp` (- (`self.levelValue`) (`self.knobTurnSpeed`)))))

(event `PedalPressed`
  ;[0 0 0] Play pedal pressed Animation
  (`|PlayMontage` (`self.SkeletalMesh`) "/Game/Assets/OverDrivePedal/Animation/anm_pedal_press_01_Montage.anm_pedal_press_01_Montage"
    (:`then`
      ;[0 0 0] Power on and off the Pedal
      (set `self.poweredOn` (not (`self.poweredOn`)))
      ;;[0 0 0] LED
      (if (`self.poweredOn`)
        (`MeshComponent.SetScalarParameterValueOnMaterials` (`self.SkeletalMesh`) "emissiveGain" (`self.Led Power`))
        (else
          (`MeshComponent.SetScalarParameterValueOnMaterials` (`self.SkeletalMesh`) "emissiveGain" 0.0))))))

(event `self.AudioCapture.OnAudioEnvelopeValue`
  (params (EnvelopeValue :type "Float (single-precision)"))
  ;[0 0 0] Audio Level
  (`AudioMixerBlueprintLibrary.GetMagnitudeForFrequencies` (`|MakeArray` 20.0 600.0 200.0 7000.0 8000.0 8000.0 11000.0 :!type "Float (single-precision)") null)
  (`SynthComponent.SetVolumeMultiplier` (`self.AudioCapture`) (* (* (`KismetMathLibrary.Conv_BoolToInt` (`self.poweredOn`)) (`self.Volume Multiplier`)) (`self.levelValue`))))

(event `KnobTurnRight`
  (set `self.levelValue` (`KismetMathLibrary.FClamp` (+ (`self.levelValue`) (`self.knobTurnSpeed`)))))

(fn `Smooth FFT`
  (params (`sample 1` :type "Float (double-precision)") (`sample 2` :type "Float (double-precision)")))

(fn `UserConstructionScript`)