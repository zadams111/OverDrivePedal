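; Audio visualizer actor that drives ShaderPlane material parameters from FFT analysis of audio output.
; BeginPlay starts output analysis, and each AudioCapture envelope event samples frequency magnitudes, feeding bass to "low" and mids to "mids".
; Every event creates two new dynamic materials, both on element 0, sourced from slots 0 and 2.
; Bass averaging and debug prints are disconnected, and SmoothFFT is an empty stub.
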(event `self.AudioCapture.OnAudioEnvelopeValue`
  (params (EnvelopeValue :type "Float (single-precision)"))
  (bind _shader_plane (`self.shader_plane`))
  (bind _shader_plane_2 (`self.shader_plane`))
  (bind _magnitudes (`AudioMixerBlueprintLibrary.GetMagnitudeForFrequencies` (`|MakeArray` 20.0 600.0 200.0 7000.0 8000.0 8000.0 11000.0 :!type "Float (single-precision)") null))
  ;[0 0 0] change a parameter based off of bass
  (bind _returnvalue (`PrimitiveComponent.CreateDynamicMaterialInstance` _shader_plane_2 0 (`PrimitiveComponent.GetMaterial` _shader_plane_2 0) "None"))
  (`MaterialInstanceDynamic.SetScalarParameterValue` _returnvalue "low" (`|GetArrayItem` _magnitudes))
  ;[0 0 0] change a parameter based off of mids
  (bind _returnvalue_2 (`PrimitiveComponent.CreateDynamicMaterialInstance` _shader_plane 0 (`PrimitiveComponent.GetMaterial` _shader_plane 2) "None"))
  (`MaterialInstanceDynamic.SetScalarParameterValue` _returnvalue_2 "mids" (`|GetArrayItem` _magnitudes 2)))

(event `self.ReceiveBeginPlay`
  ;[0 0 0] Init FFT analyzation
  (`AudioMixerBlueprintLibrary.StartAnalyzingOutput` null "VeryLarge" "NearestNeighbor"))

(fn `Smooth FFT`
  (params (`sample 1` :type "Float (double-precision)") (`sample 2` :type "Float (double-precision)")))

(fn `UserConstructionScript`)