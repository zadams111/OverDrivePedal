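; Player controller that sets up pedal input and the main UI for an overdrive pedal interaction.
; On BeginPlay it adds the IMC_Pedal Enhanced Input mapping context, then creates UI_Main and adds it to the viewport.
; When IA_PedalPress starts, it finds the first BP_OverDrivePedal in the level and calls PedalPressed on it.
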(event `self.ReceiveBeginPlay`
  (bind _returnvalue (pcsubsystem `EnhancedInputLocalPlayerSubsystem` self))
  ;[0 0 0] Add Mapping Context
  (`/Engine/EditorBlueprintResources/StandardMacros.IsValid` _returnvalue
    (:`Is Valid`
      (`EnhancedInputSubsystemInterface.AddMappingContext` _returnvalue "/Game/Inputs/IMC_Pedal.IMC_Pedal" 0 (struct))
      ;[0 0 0] UI
      (bind _returnvalue_2 (`|CreateWidget` "/Game/UI/UI_Main.UI_Main_C"))
      (bind _output_get (set `self.UI` _returnvalue_2))
      (`UserWidget.AddToViewport` _output_get 0))))

(event `EnhancedInput|/Game/Inputs/IA_PedalPress`
  (params (ActionValue :type Boolean) (ElapsedSeconds :type "Float (double-precision)") (TriggeredSeconds :type "Float (double-precision)") (InputAction :type "InputAction Object Reference" :default "/Game/Inputs/IA_PedalPress.IA_PedalPress"))
  (:`Started`
    ;[0 0 0] Press pedal
    (bind _outactors (`GameplayStatics.GetAllActorsOfClass` "/Game/Assets/OverDrivePedal/BP_OverDrivePedal.BP_OverDrivePedal_C"))
    (`/Game/Assets/OverDrivePedal/BP_OverDrivePedal.PedalPressed` (`|GetArrayItem` _outactors))))

(fn `UserConstructionScript`)